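; BP_TestPC is a test player controller for click-to-move character control using Enhanced Input and a visible cursor.
; While the move input is held, Follow traces under the cursor and paths the pawn there via SimpleMoveToLocation; release or cancel spawns a cursor effect.
; Basic attack halts movement and plays a montage with a debug print on notify.
; The Move function, a manual arrival-and-snap routine, is never called here.
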(event Input|EnhancedActionEvents|EnhancedInputActionIA_Move
  (params (ActionValue :type Boolean) (ElapsedSeconds :type Float%20%28double-precision%29) (TriggeredSeconds :type Float%20%28double-precision%29) (InputAction :type Input%20Action%20Object%20Reference :default "/Game/MyProject/Input/IA_Move.IA_Move"))
  (bind (_bishit _impactpoint) (CallFunction|CheckLand))
  (:Triggered
    (CallFunction|Follow))
  (:Started
    (AI|Navigation|StopMovement))
  (:Canceled
    (Niagara|SpawnSystematLocation "/Game/TopDown/Cursor/FX_Cursor.FX_Cursor" (select _bishit _impactpoint (Variables|Default|GetDestination)) :!label _label))
  (:Completed
    (goto _label)))

(event Input|EnhancedActionEvents|EnhancedInputActionIA_BasicAttack
  (params (ActionValue :type Boolean) (ElapsedSeconds :type Float%20%28double-precision%29) (TriggeredSeconds :type Float%20%28double-precision%29) (InputAction :type Input%20Action%20Object%20Reference :default "/Game/MyProject/Input/IA_BasicAttack.IA_BasicAttack"))
  (:Started
    (Variables|Default|SetbIsBasicAttack true)
    (Variables|Default|SetbIsMoving false)
    (AI|Navigation|StopMovement)
    (Animation|Montage|PlayMontage (Variables|/Script/Engine.Character|GetMesh (Variables|Default|GetMyPawn)) "/Game/MyProject/Animation/AM_Attack_01.AM_Attack_01" 1.0 0.0 "None" false
      (:OnNotifyBegin
        (Development|PrintString "Hello"))))
  (:Canceled
    (Variables|Default|SetbIsBasicAttack false :!label _label))
  (:Completed
    (goto _label)))

(event EventBeginPlay
  (bind _returnvalue (PlayerController|LocalPlayerSubsystems|GetEnhancedInputLocalPlayerSubsystem))
  (bind _ascharacter (Utilities|Casting|CastToCharacter (Pawn|GetControlledPawn)))
  (Variables|Default|SetMyPawn _ascharacter)
  (if (Pawn|IsLocalPlayerController)
    (Utilities|IsValid _returnvalue
      (:Is%20Valid
        (Input|AddMappingContext _returnvalue "/Game/MyProject/Input/IMC_Base.IMC_Base" 0 "(bIgnoreAllPressedKeysUntilRelease=True,bForceImmediately=False,bNotifyUserSettings=False)")
        (Input|SetInputModeGameandUI self 0 "DoNotLock" false false)))))

(event EventTick
  (params (DeltaSeconds :type Float%20%28single-precision%29)))

(fn ConstructionScript)

(fn Follow
  (bind (_bishit _impactpoint) (CallFunction|CheckLand))
  (bind _mypawn (Variables|Default|GetMyPawn))
  (if _bishit
    (Variables|Default|SetbIsMoving true)
    (bind _output_get (Variables|Default|SetDestination (Math|Vector|MakeVector (.x _impactpoint) (.y _impactpoint) (+ (.z _impactpoint) (Components|Capsule|GetUnscaledCapsuleHalfHeight (Variables|/Script/Engine.Character|GetCapsuleComponent _mypawn))))))
    (if (< 2e+01 (Math|Vector|Distance(Vector) _output_get (Transformation|GetActorLocation _mypawn)))
      (AI|Navigation|SimpleMovetoLocation self (Variables|Default|GetDestination)))))

(fn CheckLand
  (bind _array (Utilities|Array|MakeArray "ObjectTypeQuery1" "ObjectTypeQuery2"))
  (bind (_hitresult _returnvalue) (Class|PlayerController|GetHitResultUnderCursorforObjects _array true))
  (return _returnvalue (.ImpactPoint (Collision|BreakHitResult _hitresult))))

(fn Move
  (if (Variables|Default|GetbIsMoving)
    (bind _mypawn (Variables|Default|GetMyPawn)
      (:then
        (Pawn|Input|AddMovementInput _mypawn (Class|KismetMathLibrary|VectorNormal2D (Variables|/Script/Engine.MovementComponent|GetVelocity (Variables|/Script/Engine.Character|GetCharacterMovement _mypawn)) 0.0001) 1.0 false)
        (if (> 1e+01 (Math|Vector|Distance2D(Vector) (Transformation|GetActorLocation (Variables|Default|GetMyPawn)) (Variables|Default|GetDestination)))
          (AI|Navigation|StopMovement)
          (Variables|Default|SetbIsMoving false)
          (Transformation|SetActorLocation (Variables|Default|GetMyPawn) (Variables|Default|GetDestination) false false)))
      (:else))))