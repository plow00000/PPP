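; BP_TestAIC is an AI controller for BP_TestCharacter pawns.
; On possess, it runs a behavior tree only if MyPawn is already valid; otherwise it calls SetPawn without starting the tree.
; SetPawn casts the pawn to BP_TestCharacter, stores it as MyPawn and writes itself into the character's MyAIController for a two-way link.
; A Blackboard write to the Destination key is left unconnected and never runs.
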(event EventPossess
  (params (PossessedPawn :type Pawn%20Object%20Reference))
  (Variables|Default|GetMyPawn
    (:then
      (AI|RunBehaviorTree))
    (:else
      (CallFunction|SetPawn PossessedPawn))))

(fn ConstructionScript)

(fn SetPawn
  (params (Object :type Object%20Object%20Reference))
  (bind _asbp_test_character (Utilities|Casting|CastToBP_TestCharacter Object))
  (bind _output_get (Variables|Default|SetMyPawn _asbp_test_character))
  (Variables|/Game/MyProject/Framework/BP_TestCharacter.BP_TestCharacter_C|SetMyAIController _output_get self))